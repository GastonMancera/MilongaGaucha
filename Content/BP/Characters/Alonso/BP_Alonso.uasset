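; BP_Alonso is a playable side-scrolling platformer character that moves along world X, jumps and attacks through Enhanced Input.
; The attack plays an animation override and sets a flag that blocks movement, jump and further attacks until it completes or is cancelled.
; Each tick turns control rotation to face the X velocity direction and returns the character to its BeginPlay location, stored as a checkpoint, after falling below a height limit.
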(event Input|EnhancedActionEvents|EnhancedInputActionIA_Jump
  (params (ActionValue :type Boolean) (ElapsedSeconds :type Float%20%28double-precision%29) (TriggeredSeconds :type Float%20%28double-precision%29) (InputAction :type Input%20Action%20Object%20Reference :default "/Game/Assets/Control/Input/Action/IA_Jump.IA_Jump"))
  (:Triggered
    (if (not (Variables|Default|GetCheckDeAtaque))
      (Character|Jump)))
  (:Completed
    (Character|StopJumping)))

(event Input|EnhancedActionEvents|EnhancedInputActionIA_Move
  (params (ActionValue :type Float%20%28double-precision%29) (ElapsedSeconds :type Float%20%28double-precision%29) (TriggeredSeconds :type Float%20%28double-precision%29) (InputAction :type Input%20Action%20Object%20Reference :default "/Game/Assets/Control/Input/Action/IA_Move.IA_Move"))
  (if (not (Variables|Default|GetCheckDeAtaque))
    (Pawn|Input|AddMovementInput "1.000000,0.000000,0.000000" ActionValue false)))

(event Input|EnhancedActionEvents|EnhancedInputActionIA_Atack
  (params (ActionValue :type Boolean) (ElapsedSeconds :type Float%20%28double-precision%29) (TriggeredSeconds :type Float%20%28double-precision%29) (InputAction :type Input%20Action%20Object%20Reference :default "/Game/Assets/Control/Input/Action/IA_Atack.IA_Atack"))
  (:Started
    (if (not (Variables|Default|GetCheckDeAtaque))
      (|PlayAnimationOverridewithCallbacks (Class|PaperZDCharacter|GetAnimInstance) "/Game/BP/Characters/Alonso/AnimSequences/Ataque.Ataque" "DefaultSlot" 1.0 0.0
        (:then
          (Variables|Default|SetCheckDeAtaque true))
        (:OnCompleted
          (Variables|Default|SetCheckDeAtaque false :!label _label))
        (:OnCancelled
          (goto _label))))))

(event EventBeginPlay
  (|CallParentFunction)
  (bind _asplayer_controller (Utilities|Casting|CastToPlayerController (Pawn|GetController)))
  (Input|AddMappingContext (PlayerController|LocalPlayerSubsystems|GetEnhancedInputLocalPlayerSubsystem _asplayer_controller) "/Game/Assets/Control/Input/IMC_Plataformer.IMC_Plataformer" 0 "(bIgnoreAllPressedKeysUntilRelease=True,bForceImmediately=False,bNotifyUserSettings=False)")
  (Variables|Default|SetCheckPoint (Transformation|GetActorLocation)))

(event EventTick
  (params (DeltaSeconds :type Float%20%28single-precision%29))
  (|CallParentFunction DeltaSeconds)
  (CallFunction|ControlDeRotacion)
  (if (<= (.z (Transformation|GetActorLocation)) -5.7e+03)
    (Transformation|SetActorLocation (Variables|Default|GetCheckPoint) false false)))

(fn ConstructionScript
  (|CallParentFunction))

(fn ControlDeRotacion
  (bind _returnvalue (Pawn|GetController))
  (bind _returnvalue_2 (Pawn|GetController))
  (Math|Float|CompareFloat (.x (Variables|/Script/Engine.MovementComponent|GetVelocity (Variables|Character|GetCharacterMovement))) 0.0
    (:>
      (Utilities|IsValid _returnvalue
        (:Is%20Valid
          (Pawn|SetControlRotation _returnvalue (Math|Rotator|MakeRotator 0.0 0.0 0.0)))))
    (:<
      (Utilities|IsValid _returnvalue_2
        (:Is%20Valid
          (Pawn|SetControlRotation _returnvalue_2 (Math|Rotator|MakeRotator 0.0 0.0 1.8e+02)))))))